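; 2D player character for the Typhoon game that picks directional flipbook animations from its movement.
; Tick sets facing from Y velocity, then runs a jump, slide, fall, walk, idle priority chain, printing debug state.
; The jump branch is hardwired true, bypassing the timed Jumping flag from OnJumped and all later states; sliding is stubbed.
; NumPad test keys complete the stage, adjust lives or kill the player, the latter two via server-named events.
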(event `Key|NumPadNine`
  (params (Key :type "Key Structure"))
  (:`Pressed`
    (bind _astyphoon_game_state (cast `TyphoonGameState` (`GameplayStatics.GetGameState`)))
    (`TyphoonGameState.CompleteStage` _astyphoon_game_state)))

(event `Key|NumPadTwo`
  (params (Key :type "Key Structure"))
  (:`Pressed`
    (bind _astyphoon_player_state (cast `TyphoonPlayerState` (`self.PlayerState`)))
    (bind _result (`/Engine/EditorBlueprintResources/StandardMacros.IncrementInt` (`TyphoonPlayerState.GetLives` _astyphoon_player_state))
      (:`  `
        ;[1 1 1] Forcefully sets the life count on the Server. Would usually be avoided but this is just for testing.
        (`self.Set Lives On Server` _result _astyphoon_player_state)))))

(event `Set Lives On Server`
  (params (NewLives :type Integer) (PlayerState :type "TyphoonPlayerState Object Reference"))
  ;[1 1 1] Forcefully sets the life count on the Server. Would usually be avoided but this is just for testing.
  (`TyphoonPlayerState.SetLives` PlayerState NewLives))

(event `Key|NumPadOne`
  (params (Key :type "Key Structure"))
  (:`Pressed`
    (bind _astyphoon_player_state (cast `TyphoonPlayerState` (`self.PlayerState`)))
    (bind _result (`/Engine/EditorBlueprintResources/StandardMacros.DecrementInt` (`TyphoonPlayerState.GetLives` _astyphoon_player_state))
      (:`  `
        ;[1 1 1] Forcefully sets the life count on the Server. Would usually be avoided but this is just for testing.
        (`self.Set Lives On Server` _result _astyphoon_player_state)))))

(event `Kill Player On Server`
  (params (`Player State` :type "TyphoonPlayerState Object Reference"))
  ;[1 1 1] Forcefully sets the life count on the Server. Would usually be avoided but this is just for testing.
  (`TyphoonPlayerState.KillPlayer` `Player State`))

(event `Key|NumPadThree`
  (params (Key :type "Key Structure"))
  (:`Pressed`
    (bind _astyphoon_player_state (cast `TyphoonPlayerState` (`self.PlayerState`)))
    ;[1 1 1] Forcefully sets the life count on the Server. Would usually be avoided but this is just for testing.
    (`self.Kill Player On Server` _astyphoon_player_state)))

(event `self.OnJumped`
  ;[1 1 1] Tells character that it should be playing the jump animation
  (set `self.bJumping` true)
  (`KismetSystemLibrary.RetriggerableDelay` (`self.JumpAnimationDuration`))
  (set `self.bJumping` false))

(event `self.ReceiveTick`
  (params (DeltaSeconds :type "Float (single-precision)"))
  (bind _character_flipbook (`self.Character FlipBook`))
  (bind _character_flipbook_2 (`self.Character FlipBook`))
  (bind _character_flipbook_3 (`self.Character FlipBook`))
  (bind _character_flipbook_4 (`self.Character FlipBook`))
  (`|ExecutionSequence`
    (:`then_0`
      ;[1 1 1] Update Look Position
      (bind _value (`self.GetIsMovingLeft`))
      (if _value
        (set `self.bLookingRight` false)
        (else
          (bind _value_2 (`self.GetIsMovingRight`))
          (if _value_2
            (set `self.bLookingRight` true)))))
    (:`then_1`
      ;[1 1 1] Jumping
      (`self.GetIsJumping`)
      (if true
        (if (`self.bLookingRight`)
          (`PaperFlipbookComponent.SetFlipbook` _character_flipbook_4 "/Game/Flipbooks/Right/RightJump.RightJump")
          (else
            (`PaperFlipbookComponent.SetFlipbook` _character_flipbook_4 "/Game/Flipbooks/Left/LeftJump.LeftJump")))
        (else
          ;[1 1 1] Sliding - Not yet implemented
          (bind _value_3 (`self.GetIsSliding`))
          (if _value_3
            (if (`self.bLookingRight`)
              (`PaperFlipbookComponent.SetFlipbook` _character_flipbook "/Game/Flipbooks/Right/RightSlide.RightSlide")
              (else
                (`PaperFlipbookComponent.SetFlipbook` _character_flipbook "/Game/Flipbooks/Left/LeftSlide.LeftSlide")))
            (else
              ;[1 1 1] Falling
              (bind _value_4 (`self.GetIsFalling`))
              (if _value_4
                (if (`self.bLookingRight`)
                  (`PaperFlipbookComponent.SetFlipbook` _character_flipbook_3 "/Game/Flipbooks/Right/RightFall.RightFall")
                  (else
                    (`PaperFlipbookComponent.SetFlipbook` _character_flipbook_3 "/Game/Flipbooks/Left/LeftFall.LeftFall")))
                (else
                  ;[1 1 1] Walking Left
                  (bind _value_5 (`self.GetIsMovingLeft`))
                  (if _value_5
                    (`PaperFlipbookComponent.SetFlipbook` (`self.Character FlipBook`) "/Game/Flipbooks/Left/LeftWalk.LeftWalk")
                    (else
                      ;[1 1 1] Walking Right
                      (bind _value_6 (`self.GetIsMovingRight`))
                      (if _value_6
                        (`PaperFlipbookComponent.SetFlipbook` (`self.Character FlipBook`) "/Game/Flipbooks/Right/RightWalk.RightWalk")
                        (else
                          ;[1 1 1] Idle
                          (if (`self.bLookingRight`)
                            (`PaperFlipbookComponent.SetFlipbook` _character_flipbook_2 "/Game/Flipbooks/Right/RightIdle.RightIdle")
                            (else
                              (`PaperFlipbookComponent.SetFlipbook` _character_flipbook_2 "/Game/Flipbooks/Left/LeftIdle.LeftIdle"))))))))))))))
    (:`then_2`
      (`KismetSystemLibrary.PrintString` (`KismetTextLibrary.Conv_TextToString` (`|FormatText` "Looking {Direction}" (`self.bLookingRight`))))
      (`KismetSystemLibrary.PrintString` (`KismetTextLibrary.Conv_TextToString` (`|FormatText` "Jumping: {Value}" (`self.bJumping`)))))))

(fn `GetIsFalling`
  (returns (Value :type Boolean))
  (return (`|EnumEquality` (`CharacterMovementComponent.MovementMode` (`self.CharacterMovement`)) "MOVE_Falling")))

(fn `GetIsJumping`
  (returns (Value :type Boolean))
  (return (`self.bJumping`)))

(fn `GetIsMovingLeft`
  (returns (Value :type Boolean))
  (bind (_returnvalue_x _returnvalue_y) (`KismetMathLibrary.BreakVector` (`self.GetVelocity`)))
  (return (> _returnvalue_y 0.0)))

(fn `GetIsMovingRight`
  (returns (Value :type Boolean))
  (bind (_returnvalue_x _returnvalue_y) (`KismetMathLibrary.BreakVector` (`self.GetVelocity`)))
  (return (< _returnvalue_y 0.0)))

(fn `GetIsSliding`
  (returns (Value :type Boolean))
  (return false))

(fn `GetNoHorizontalMovement`
  (returns (Value :type Boolean))
  (bind (_returnvalue_x _returnvalue_y) (`KismetMathLibrary.BreakVector` (`self.GetVelocity`)))
  (return (== _returnvalue_y 0.0)))

(fn `UserConstructionScript`)