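; BP_TyphoonCharacter is a character Blueprint whose event graph holds numpad debug keys for testing player lives and death.
; Keys One, Two and Three lower lives, raise lives or kill the player through the TyphoonPlayerState.
; They route through SetLivesOnServer and KillPlayerOnServer events, deliberately forcing changes on the server for testing.
; Key Nine only casts the game state, and the construction script is empty.
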(event `Key|NumPadNine`
  (params (Key :type "Key Structure"))
  (:`Pressed`
    (cast `TyphoonGameState` (`GameplayStatics.GetGameState`))))

(event `Key|NumPadTwo`
  (params (Key :type "Key Structure"))
  (:`Pressed`
    (bind _astyphoon_player_state (cast `TyphoonPlayerState` (`self.PlayerState`)))
    (bind _result (`/Engine/EditorBlueprintResources/StandardMacros.IncrementInt` (`TyphoonPlayerState.GetLives` _astyphoon_player_state))
      (:`  `
        ;[1 1 1] Forcefully sets the life count on the Server. Would usually be avoided but this is just for testing.
        (`self.Set Lives On Server` _result _astyphoon_player_state)))))

(event `Set Lives On Server`
  (params (NewLives :type Integer) (PlayerState :type "TyphoonPlayerState Object Reference"))
  ;[1 1 1] Forcefully sets the life count on the Server. Would usually be avoided but this is just for testing.
  (`TyphoonPlayerState.SetLives` PlayerState NewLives))

(event `Key|NumPadOne`
  (params (Key :type "Key Structure"))
  (:`Pressed`
    (bind _astyphoon_player_state (cast `TyphoonPlayerState` (`self.PlayerState`)))
    (bind _result (`/Engine/EditorBlueprintResources/StandardMacros.DecrementInt` (`TyphoonPlayerState.GetLives` _astyphoon_player_state))
      (:`  `
        ;[1 1 1] Forcefully sets the life count on the Server. Would usually be avoided but this is just for testing.
        (`self.Set Lives On Server` _result _astyphoon_player_state)))))

(event `Kill Player On Server`
  (params (`Player State` :type "TyphoonPlayerState Object Reference"))
  ;[1 1 1] Forcefully sets the life count on the Server. Would usually be avoided but this is just for testing.
  (`TyphoonPlayerState.KillPlayer` `Player State`))

(event `Key|NumPadThree`
  (params (Key :type "Key Structure"))
  (:`Pressed`
    (bind _astyphoon_player_state (cast `TyphoonPlayerState` (`self.PlayerState`)))
    ;[1 1 1] Forcefully sets the life count on the Server. Would usually be avoided but this is just for testing.
    (`self.Kill Player On Server` _astyphoon_player_state)))

(fn `UserConstructionScript`)