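; Cannonball projectile that kills any player pawn it hits.
; The first component hit sets a guard flag, then calls KillPlayer on the hit pawn's TyphoonPlayerState, if it has one.
; Any hit also stops physics, hides the shape, swaps particle effects and plays audio before destroying the actor after a short delay.
; Exceeding its lifetime destroys it immediately, and the construction script assigns Shape as the ProjectileMesh.
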(event `self.Shape.OnComponentHit`
  (params (HitComponent :type "PrimitiveComponent Object Reference") (OtherActor :type "Actor Object Reference") (OtherComp :type "PrimitiveComponent Object Reference") (NormalImpulse :type "Vector Structure") (Hit :type "HitResult Structure (by ref)"))
  (bind _shape (`self.Shape`))
  (if (not (`self.BeingDestroyed`))
    (set `self.BeingDestroyed` true)
    (`|ExecutionSequence`
      (:`then_0`
        (bind _aspawn (cast `Pawn` OtherActor))
        (bind _astyphoon_player_state (cast `TyphoonPlayerState` (`Pawn.PlayerState` _aspawn)))
        (`TyphoonPlayerState.KillPlayer` _astyphoon_player_state))
      (:`then_1`
        (`PrimitiveComponent.SetSimulatePhysics` _shape false)
        (`SceneComponent.SetVisibility` _shape false false)
        (`ActorComponent.Activate` (`self.ParticleSystem1`) false)
        (`AudioComponent.Play` (`self.Audio`) 0.0)
        (`ActorComponent.K2_DestroyComponent` (`self.ParticleSystem`))
        (`KismetSystemLibrary.Delay` 1.0)
        (`self.K2_DestroyActor`)))))

(event `self.OnLifetimeExceeded`
  (`self.K2_DestroyActor`))

(fn `UserConstructionScript`
  (set `self.ProjectileMesh` (`self.Shape`)))