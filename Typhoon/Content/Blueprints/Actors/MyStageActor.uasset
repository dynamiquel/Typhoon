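; MyStageActor is a stage actor with a pickup component that reacts to stage play and hide events.
; On play it enables query and physics collision on Cube and query-only collision on Box; on hide it disables both.
; The construction script assigns Box as the Pickup component's collider, and the pickup event only prints the collecting pawn's display name.
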(event `self.OnStagePlay`
  (`PrimitiveComponent.SetCollisionEnabled` (`self.Cube`) "QueryAndPhysics")
  (`PrimitiveComponent.SetCollisionEnabled` (`self.Box`) "QueryOnly"))

(event `self.OnStageHide`
  (`PrimitiveComponent.SetCollisionEnabled` (`self.Cube`) "NoCollision")
  (`PrimitiveComponent.SetCollisionEnabled` (`self.Box`) "NoCollision"))

(event `self.Pickup.OnPickup`
  (params (Pawn :type "Pawn Object Reference"))
  (`KismetSystemLibrary.PrintString` (`KismetSystemLibrary.GetDisplayName` Pawn)))

(fn `UserConstructionScript`
  (set `PickupComponent.Collider` (`self.Box`) (`self.Pickup`)))