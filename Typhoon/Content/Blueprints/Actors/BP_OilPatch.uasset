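; BP_OilPatch is a hazard actor that makes TyphoonCharacters slow and slippery while they overlap its Box.
; On begin overlap it cuts walk speed relative to the character's initial value, removes ground friction and overrides braking deceleration and acceleration.
; On end overlap it calls the character's ResetSpeed to restore normal movement.
; It edits CharacterMovement directly because physical materials were not being detected.
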(event `self.Box.OnComponentEndOverlap`
  (params (OverlappedComponent :type "PrimitiveComponent Object Reference") (OtherActor :type "Actor Object Reference") (OtherComp :type "PrimitiveComponent Object Reference") (OtherBodyIndex :type Integer))
  ;[1 1 1] Essentially reset character movement to normal
  (bind _astyphoon_character (cast `TyphoonCharacter` OtherActor))
  (`TyphoonCharacter.ResetSpeed` _astyphoon_character))

(event `self.Box.OnComponentBeginOverlap`
  (params (OverlappedComponent :type "PrimitiveComponent Object Reference") (OtherActor :type "Actor Object Reference") (OtherComp :type "PrimitiveComponent Object Reference") (OtherBodyIndex :type Integer) (bFromSweep :type Boolean) (SweepResult :type "HitResult Structure (by ref)"))
  (bind _astyphoon_character (cast `TyphoonCharacter` OtherActor))
  (bind _charactermovement (`Character.CharacterMovement` _astyphoon_character))
  (set `CharacterMovementComponent.MaxWalkSpeed` (* (`TyphoonCharacter.InitialMaxWalkSpeed` _astyphoon_character) 0.7) _charactermovement)
  (set `CharacterMovementComponent.GroundFriction` 0.0 _charactermovement)
  (set `CharacterMovementComponent.BrakingDecelerationWalking` 200.0 _charactermovement)
  (set `CharacterMovementComponent.MaxAcceleration` 400.0 _charactermovement))

(fn `UserConstructionScript`)