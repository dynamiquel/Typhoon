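; BP_HealthPickup is a pickup actor that grants one extra life to the Typhoon character that collects it.
; The construction script assigns a box as the Pickup component's collider, and its OnPickup event increments Lives on the character's TyphoonPlayerState.
; A Destroying flag blocks repeat triggers while the mesh is removed, audio and particles play, and the actor destroys itself after a short delay.
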(event `self.Pickup.OnPickup`
  (params (Pawn :type "Pawn Object Reference"))
  (if (not (`self.bDestroying`))
    (bind _astyphoon_character (cast `TyphoonCharacter` Pawn))
    (set `self.bDestroying` true)
    (bind _astyphoon_player_state (cast `TyphoonPlayerState` (`Pawn.PlayerState` _astyphoon_character)))
    (`TyphoonPlayerState.SetLives` _astyphoon_player_state (+ (`TyphoonPlayerState.GetLives` _astyphoon_player_state) 1))
    (`ActorComponent.K2_DestroyComponent` (`self.StaticMesh`))
    (`AudioComponent.Play` (`self.Audio`) 0.0)
    (`ActorComponent.Activate` (`self.ParticleSystem`) false)
    (`KismetSystemLibrary.Delay` 1.0)
    (`self.K2_DestroyActor`)))

(fn `UserConstructionScript`
  (set `PickupComponent.Collider` (`self.Box`) (`self.Pickup`)))