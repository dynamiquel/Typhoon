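; Turret actor Blueprint that picks a target by AI sight and plays audio when it fires.
; UpdateTarget takes the first sight-perceived actor as CurrentTarget, keeps the existing target if that actor is a spectator, and clears it when none are perceived.
; The construction script sets the Arrow component as BulletSpawnPoint; aiming and projectile logic are not in these graphs.
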(event `self.UpdateTarget`
  (bind _outactors (`AIPerceptionComponent.GetKnownPerceivedActors` (`self.AIPerception`) "/Script/AIModule.AISense_Sight"))
  (bind _output (`|GetArrayItem` _outactors))
  (if (> (`KismetArrayLibrary.Array_Length` _outactors) 0)
    (cast `/Game/Blueprints/Pawns/BP_Spectator` _output ; Ignores the spectator actor
      (:`CastFailed`
        (set `self.CurrentTarget` _output)))
    (elif (`KismetSystemLibrary.IsValid` (`self.CurrentTarget`))
      (set `self.CurrentTarget` null))))

(event `self.OnFire`
  (`AudioComponent.Play` (`self.Audio`) 0.0))

(fn `UserConstructionScript`
  (set `self.BulletSpawnPoint` (`self.Arrow`)))