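; BP_TyphoonPlayerController is a player controller that manages the HUD, soundtrack and end-of-game screens.
; BeginPlay adds the HUD to the player's screen and starts the music.
; OnGameOver shows a won or game-over widget with UI-only input and cursor, then pauses, delayed on a win and immediately with a sound on a loss.
; A pause-menu toggle exists but is unwired, so it never runs.
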(event `Key|G`
  (params (Key :type "Key Structure")))

(event `Key|Escape`
  (params (Key :type "Key Structure")))

(event `self.ReceiveBeginPlay`
  (bind _returnvalue (`|CreateWidget` "/Game/Blueprints/Widgets/WBP_Hud.WBP_Hud_C" self))
  (`UserWidget.AddToPlayerScreen` _returnvalue 10)
  (`GameplayStatics.PlaySound2D` "/Game/Soundtrack_Cue.Soundtrack_Cue" 1.0 1.0 0.0 null null))

(event `self.OnGameOver`
  (params (GameWon :type Boolean))
  (if GameWon
    (bind _returnvalue (`|CreateWidget` "/Game/Blueprints/Widgets/WBP_GameWon.WBP_GameWon_C" self))
    (`WidgetBlueprintLibrary.SetInputMode_UIOnlyEx` self _returnvalue)
    (set `self.bShowMouseCursor` true)
    (`UserWidget.AddToViewport` _returnvalue 100)
    (`KismetSystemLibrary.Delay` 2.0)
    (`GameplayStatics.SetGamePaused` true)
    (else
      (bind _returnvalue_2 (`|CreateWidget` "/Game/Blueprints/Widgets/WBP_GameOver.WBP_GameOver_C" self))
      (`WidgetBlueprintLibrary.SetInputMode_UIOnlyEx` self _returnvalue_2)
      (set `self.bShowMouseCursor` true)
      (`UserWidget.AddToViewport` _returnvalue_2 100)
      (`GameplayStatics.SetGamePaused` true)
      (`GameplayStatics.PlaySound2D` "/Game/Game_Over_Cue.Game_Over_Cue" 1.0 1.0 0.0 null null))))

(fn `UserConstructionScript`)