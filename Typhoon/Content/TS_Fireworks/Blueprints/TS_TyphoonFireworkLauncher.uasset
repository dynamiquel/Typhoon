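; Firework launcher Blueprint that fires a shell when the game is won.
; Each tick it casts the game state to TyphoonGameState and checks the game-won flag, using a Started boolean so LaunchShell is called only once.
; BeginPlay, overlap and construction script add no logic of their own.
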(event `self.ReceiveTick`
  (params (DeltaSeconds :type "Float (single-precision)"))
  (bind _astyphoon_game_state (cast `TyphoonGameState` (`GameplayStatics.GetGameState`)))
  (if (and (not (`self.Started`)) (`TyphoonGameState.GetGameWon` _astyphoon_game_state))
    (set `self.Started` true)
    (`self.LaunchShell`)))

(fn `UserConstructionScript`
  (`parent.UserConstructionScript`))